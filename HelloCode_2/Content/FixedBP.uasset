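; FixedBP is an overlap test actor that shows a greeting or farewell naming the other actor.
; MyonBeginOverlap and MyonEndOverlap set the Text object to "Hello" or "Bye" joined to that actor's object name.
; The default BeginPlay, ActorBeginOverlap and Tick events, the construction script and MakeText are empty, and nothing in these graphs calls or binds the two overlap events.
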(event EventBeginPlay)

(event Collision|EventActorBeginOverlap
  (params (OtherActor :type Actor%20Object%20Reference)))

(event EventTick
  (params (DeltaSeconds :type Float%20%28single-precision%29)))

(event EventMyonBeginOverlap
  (params (OverlappedActor :type Actor%20Object%20Reference) (OtherActor :type Actor%20Object%20Reference))
  (Rendering|Components|TextRender|SetText (Variables|Default|GetText) (Utilities|Text|ToText(String) (Utilities|String|Append "Hello " (Utilities|GetObjectName OtherActor)))))

(event EventMyonEndOverlap
  (params (OverlappedActor :type Actor%20Object%20Reference) (OtherActor :type Actor%20Object%20Reference))
  (Rendering|Components|TextRender|SetText (Variables|Default|GetText) (Utilities|Text|ToText(String) (Utilities|String|Append "Bye " (Utilities|GetObjectName OtherActor)))))

(fn ConstructionScript)

(fn MakeText)